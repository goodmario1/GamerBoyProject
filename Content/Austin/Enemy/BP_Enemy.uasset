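; BP_Enemy is an enemy that switches between roaming and following the player based on AI perception.
; Sensing the player pawn requests the follow state through the ACStateMachine component and clears any pending lose-sight timer.
; Losing the player starts a two-second one-shot timer that requests a return to roaming, so brief breaks in perception do not end the chase.
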(event OnTargetPerceptionUpdated(AIPerception)
  (params (Actor :type Actor%20Object%20Reference) (Stimulus :type AI%20Stimulus%20Structure))
  (if (== Actor (Game|Player|GetPlayerPawn 0))
    (if (.bSuccessfullySensed (Utilities|Struct|BreakAIStimulus Stimulus))
      (CallFunction|ChangeState "/Game/Austin/Enemy/OverworldStates/AC_State_Follow.AC_State_Follow_C")
      (Utilities|Time|ClearandInvalidateTimerbyHandle (stale _returnvalue))
      (else
        (bind _returnvalue (Utilities|Time|SetTimerbyEvent (delegate Custom|Hasn'tSeenPlayerInAwhile) 2.0))))))

(event Custom|Hasn'tSeenPlayerInAwhile
  (CallFunction|ChangeState "/Game/Austin/Enemy/OverworldStates/AC_State_Roam.AC_State_Roam_C"))

(event EventChangeState
  (params (NextState :type AC%20Base%20State%20Class%20Reference))
  (Default|TryChangingtoState (Variables|Default|GetAC_StateMachine) NextState))

(fn ConstructionScript)