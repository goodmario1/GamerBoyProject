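; Overworld enemy state component that makes its owning enemy follow the player.
; On entering the state it runs the parent logic, then issues a SimpleMoveToActor through the owner's AI controller.
; The main behavior reissues that move whenever the owner is more than 300 units from the player pawn.
; The move's goal is the player controller, while the distance check uses the pawn.
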(event EventRunMainBehavior
  (|CallParentFunction)
  (if (> (Transformation|GetDistanceTo (Components|GetOwner) (Game|Player|GetPlayerPawn 0)) 3e+02)
    (CallFunction|GotoPlayer)))

(event EventEnterState
  (|CallParentFunction)
  (CallFunction|GotoPlayer))

(fn GotoPlayer
  (AI|Navigation|SimpleMovetoActor (AI|GetAIController (Components|GetOwner)) (Game|GetPlayerController 0))
  (return))