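; Actor component state machine for overworld enemies that runs one AC_BaseState component at a time, starting in the Roam state.
; On BeginPlay it maps the owner's state components by class and forwards the owner's overlap events to the current state.
; Change requests queue a NextState, which Tick applies by exiting and entering states, otherwise ticking the current one.
; It also keeps the previous state for restoring and prints warnings for missing states.
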(event Custom|SetInitialState
  (params (StateClass :type AC%20Base%20State%20Class%20Reference))
  (Variables|Default|GetCurrentState
    (:then
      (Development|PrintString "SetInitialState can only be called once per actor" true true "(R=1.000000,G=0.027276,B=0.000000,A=1.000000)" 1e+01))
    (:else
      (bind _value (Utilities|CheckMapKey StateClass)
        (:Out
          (bind _output_get (Variables|Default|SetCurrentState _value))
          (Default|EnterState _output_get))))))

(event Custom|TryChangingToState
  (params (NextState :type AC%20Base%20State%20Class%20Reference))
  (if (== NextState 0)
    (Development|PrintString "Just tried changing to state: none, make sure to use the dropdown to specify which state to change to" true true "(R=1.000000,G=0.000000,B=0.197871,A=1.000000)" 5.0)
    (else
      (bind _value (Utilities|CheckMapKey NextState)
        (:Out
          (bind _output_get (Variables|Default|SetNextState _value))
          (Development|PrintString (Utilities|String|Append "Agent changing state to " (Utilities|GetDisplayName _output_get))))))))

(event Custom|RestorepreviousState
  (Utilities|IsValid (Variables|Default|GetPrevState)
    (:Is%20Valid
      (Variables|Default|SetNextState (Variables|Default|GetPrevState)))
    (:Is%20Not%20Valid
      (Development|PrintString "Attempted to restore previous state but still on the initial state" true true "(R=1.000000,G=0.000000,B=0.046856,A=1.000000)"))))

(event EventBeginPlay
  (|BindCollisionsGraph)
  (CallFunction|BuildStatesLibrary)
  (CallFunction|SetInitialState "/Game/Austin/Enemy/OverworldStates/AC_State_Roam.AC_State_Roam_C"))

(event EventTick
  (params (DeltaSeconds :type Float%20%28single-precision%29))
  (Utilities|IsValid (Variables|Default|GetNextState)
    (:Is%20Valid
      (Default|ExitState (Variables|Default|GetCurrentState))
      (Variables|Default|SetPrevState (Variables|Default|GetCurrentState))
      (bind _output_get (Variables|Default|SetCurrentState (Variables|Default|GetNextState)))
      (Default|EnterState _output_get)
      (Variables|Default|SetNextState 0))
    (:Is%20Not%20Valid
      (Utilities|IsValid (Variables|Default|GetCurrentState)
        (:Is%20Valid
          (Default|TickState (Variables|Default|GetCurrentState)))
        (:Is%20Not%20Valid
          (Development|PrintString "Current State isn't set, did you remember to set an initial state?" true true "(R=1.000000,G=0.000000,B=0.050567,A=1.000000)"))))))

(fn BuildStatesLibrary
  (for _array_element (Actor|GetComponentsByClass (Components|GetOwner) "/Game/Austin/Enemy/OverworldStates/AC_BaseState.AC_BaseState_C")
    (Utilities|Map|Add (Variables|Default|GetAllStates) (Utilities|GetClass _array_element) _array_element)))

(fn IsCurrentState
  (params (StateClass :type AC%20Base%20State%20Class%20Reference))
  (return (== StateClass (Utilities|GetClass (Variables|Default|GetCurrentState)))))

(event Custom|ActorBeginOverlap
  (params (OverlappedActor :type Actor%20Object%20Reference) (OtherActor :type Actor%20Object%20Reference))
  (Default|EventBeginOverlapState (Variables|Default|GetCurrentState) OtherActor))

(event Custom|ActorEndOverlap
  (params (OverlappedActor :type Actor%20Object%20Reference) (OtherActor :type Actor%20Object%20Reference))
  (Default|EndOverlapState (Variables|Default|GetCurrentState) OtherActor))