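; Idle state component for an overworld enemy's state machine.
; On entry it runs the parent state logic and stops the owner's AI controller movement.
; On tick, once more than two seconds have passed since entry, it tells the owner to switch to the Roam state.
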(event EventEnter
  (|CallParentFunction)
  (AI|Navigation|StopMovement (AI|GetAIController (Components|GetOwner))))

(event EventTickState
  (if (> (- (Utilities|Time|GetTimeSeconds) (Variables|Default|GetTimeEntered)) 2.0)
    (Class|IMachine|ChangeStates(Message) (Components|GetOwner) "/Game/Austin/Enemy/OverworldStates/AC_State_Roam.AC_State_Roam_C")))