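; Overworld enemy roam state component that patrols the owner through an array of nav points.
; On entering, it skips the current point if the owner already overlaps it, then sends the AI controller toward the selected point.
; Overlapping that point advances the index, wrapping to zero, and switches the owner to the idle state.
; An unassigned nav point prints a warning.
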(event EventEnterState
  (|CallParentFunction)
  (CallFunction|PreventNavigatingifAlreadyatGoal)
  (AI|Navigation|SimpleMovetoActor (AI|GetAIController (Components|GetOwner)) (CallFunction|GetCurrentNavPoint)))

(event EventEventBeginOverlapState
  (params (Other%20Actor :type Actor%20Object%20Reference))
  (if (== Other%20Actor (CallFunction|GetCurrentNavPoint))
    (CallFunction|ChooseNextNavPoint)))

(fn PreventNavigatingifAlreadyatGoal
  (bind _array_element (Utilities|Array|ForEachLoopwithBreak (Collision|GetOverlappingActors (Components|GetOwner) 0 :!class /Script/Engine.Actor) :!label _label)
    (:LoopBody
      (if (== _array_element (CallFunction|GetCurrentNavPoint))
        (CallFunction|ChooseNextNavPoint)
        (goto _label Break)))))

(fn GetCurrentNavPoint
  (bind _mynavpoints (Variables|Default|GetmyNavPoints))
  (bind _selectedindex (Variables|Default|GetSelectedIndex))
  (bind _output (Utilities|Array|Get(acopy) _mynavpoints _selectedindex))
  (Utilities|IsValid _output
    (:Is%20Valid
      (return _output))
    (:Is%20Not%20Valid
      (Development|PrintString (Utilities|String|Append (Utilities|GetDisplayName (Components|GetOwner)) " Just tried to access an invalid nav point, make sure the patrol component has these assigned in the level editor") true true "(R=1.000000,G=0.034709,B=0.000000,A=1.000000)"))))

(fn ChooseNextNavPoint
  (bind _result (Math|Integer|IncrementInt (Variables|Default|GetSelectedIndex))
    (:%20%20
      (if (Utilities|Array|IsValidIndex (Variables|Default|GetmyNavPoints) _result)
        _
        (else
          (Variables|Default|SetSelectedIndex 0)))
      (Class|INavAgent|ChangeState(Message) (Components|GetOwner) "/Game/Austin/Enemy/OverworldStates/AC_State_Idle.AC_State_Idle_C"))))