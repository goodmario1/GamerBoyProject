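; Battle player character that runs a timed key-press quick time event, with damage outcomes only printed as debug strings.
; CreateQTE shows a prompt widget, zeroes max acceleration and drains the timer bar with a timeline rate-scaled to the requested duration.
; The correct key in the bar's last quarter prints crit damage; earlier presses or timeout print normal damage.
; BeginPlay disables movement; ending a QTE restores only acceleration.
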(event Custom|CreateQTE
  (params (TargetKey :type Key%20Structure :default "None") (Duration :type Float%20%28double-precision%29))
  ;[1 1 1] So they can't leave before completing QTE
  (Variables|/Script/Engine.CharacterMovementComponent|SetMaxAcceleration (Variables|Character|GetCharacterMovement) 0.0)
  ;[1 1 1] Create QTE Widget, make a reference and put it on-screen
  (bind _returnvalue (UserInterface|CreateWidget "/Game/Alex/WBP_QTE_Test.WBP_QTE_Test_C"))
  (bind _output_get (Variables|Default|SetQteWidgetReference _returnvalue))
  (UserInterface|Viewport|AddtoViewport _output_get 0)
  ;[1 1 1] Get the InputKey as Text for Widget text
  (Default|SetQTEText (Variables|Default|GetQteWidgetReference) (Class|KismetInputLibrary|KeyGetDisplayName TargetKey true))
  ;[1 1 1] Grab the key from event and set it as a Key value
  (Variables|Default|SetInputKey TargetKey)
  ;[1 1 1] Set Input Key Event in progress
  (Variables|Default|SetInputKeyEventInProgress? true)
  ;[1 1 1] Example: 1/2=0.5 The 1 second TL plays at half speed (2 seconds)
  (Components|Timeline|SetPlayRate (Variables|Default|GetTL_Duration) (/ 1.0 Duration))
  ;[1 1 1] Can't do TLs in AC :(
  (bind _value (Timeline|TL_Duration PlayFromStart)
    (:Update
      ;[1 1 1] Access TimerBar and decrease its percent
      (Progress|SetPercent (Variables|/Game/Alex/WBP_QTE_Test.WBP_QTE_Test_C|GetTimerBar (Variables|Default|GetQteWidgetReference)) (Math|Float|Lerp 1.0 0.0 _value)))
    (:Finished
      ;[1 1 1] Was the Input Key Event finished before the TL finished? If not, print "normal damage"
      (if (Variables|Default|GetInputKeyEventInProgress?)
        (Development|PrintString "Normal Damage"))
      ;[1 1 1] After TL ended, Input Key Event is no longer in progress
      (Variables|Default|SetInputKeyEventInProgress? false)
      (Widget|RemovefromParent (Variables|Default|GetQteWidgetReference))
      ;[1 1 1] Re-enable Movement after TL finishes
      (Variables|/Script/Engine.CharacterMovementComponent|SetMaxAcceleration (Variables|Character|GetCharacterMovement) 2048.0))))

(event EventBeginPlay
  (Pawn|Components|CharacterMovement|DisableMovement (Variables|Character|GetCharacterMovement)))

(event Input|KeyboardEvents|AnyKey
  (params (Key :type Key%20Structure :default "None"))
  (:Pressed
    ;[1 1 1] Is the Input Key Event in progress?
    (if (Variables|Default|GetInputKeyEventInProgress?)
      ;[1 1 1] Has the Correct Input Key been pressed?
      (if (== Key (Variables|Default|GetInputKey))
        ;[1 1 1] Is the InputKey being pressed when the TimerBar's percent below or equal to 25%? If yes, print "Crit Damage". If no, print "Normal Damage"
        (if (<= (Variables|/Script/UMG.ProgressBar|GetPercent (Variables|/Game/Alex/WBP_QTE_Test.WBP_QTE_Test_C|GetTimerBar (Variables|Default|GetQteWidgetReference))) 0.25)
          (Development|PrintString "Crit Damage")
          (else
            (Development|PrintString "Normal Damage")))
        ;[1 1 1] After player attempted QTE, Input Key Event is no longer in progress
        (Variables|Default|SetInputKeyEventInProgress? false)
        (Widget|RemovefromParent (Variables|Default|GetQteWidgetReference))
        ;[1 1 1] Re-enable movement after attempting QTE event
        (Variables|/Script/Engine.CharacterMovementComponent|SetMaxAcceleration (Variables|Character|GetCharacterMovement) 2048.0)))))

(fn ConstructionScript
  (|CallParentFunction))