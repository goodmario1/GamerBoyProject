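; Player character for the battle level, with movement disabled on BeginPlay and a quick-time event (QTE) prototype.
; CreateQTE is empty; its unwired logic would show a key-prompt widget whose bar drains on a timeline scaled to Duration.
; The correct key prints crit damage in the bar's last quarter, otherwise normal damage, as does a timeout in the unwired logic.
; P loads MainLevel.
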(event Custom|CreateQTE
  (params (TargetKey :type Key%20Structure :default "None") (Duration :type Float%20%28double-precision%29)))

(event EventBeginPlay
  (Pawn|Components|CharacterMovement|DisableMovement (Variables|Character|GetCharacterMovement)))

(event Input|KeyboardEvents|AnyKey
  (params (Key :type Key%20Structure :default "None"))
  (:Pressed
    ;[1 0.491 0.4793] Is the Input Key Event in progress?
    (if (Variables|Default|GetInputKeyEventInProgress?)
      ;[1 0.491 0.4793] Has the Correct Input Key been pressed?
      (if (== Key (Variables|Default|GetInputKey))
        ;[1 0.491 0.4793] Is the InputKey being pressed when the TimerBar's percent below or equal to 25%? If yes, print "Crit Damage". If no, print "Normal Damage"
        (if (<= (Variables|/Script/UMG.ProgressBar|GetPercent (Variables|/Game/Alex/WBP_CommonActivatableQTE_Test.WBP_CommonActivatableQTE_Test_C|GetTimerBar (Variables|Default|GetCommonQteWidgetReference))) 0.25)
          (Development|PrintString "Crit Damage")
          (else
            (Development|PrintString "Normal Damage")))
        ;[1 0.491 0.4793] After player attempted QTE, Input Key Event is no longer in progress
        (Variables|Default|SetInputKeyEventInProgress? false)
        (Class|CommonActivatableWidget|DeactivateWidget (Variables|Default|GetCommonQteWidgetReference))
        ;[0.6867 1 0.6172] Re-enable movement after attempting QTE event
        (Variables|/Script/Engine.CharacterMovementComponent|SetMaxAcceleration (Variables|Character|GetCharacterMovement) 2048.0)))))

(event Input|KeyboardEvents|P
  (params (Key :type Key%20Structure :default "None"))
  (:Pressed
    (Game|OpenLevel(byName) "MainLevel")
    (Development|PrintString "Overworld Loaded")))

(fn ConstructionScript
  (|CallParentFunction))