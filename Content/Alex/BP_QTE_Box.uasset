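; BP_QTE_Box is a trigger actor that starts a quick time event when the Alex player character overlaps it.
; On begin overlap it casts to BP_PlayerCharacter_Alex, stores the reference and calls its CreateQTE with the Z key and a random short duration.
; When that character leaves the overlap, it deactivates the character's common QTE widget.
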(event EventBeginPlay)

(event Collision|EventActorBeginOverlap
  (params (OtherActor :type Actor%20Object%20Reference))
  (bind _asbp_player_character_alex (Utilities|Casting|CastToBP_PlayerCharacter_Alex OtherActor))
  (Variables|Default|SetPlayerCharacterAlexReference _asbp_player_character_alex)
  (if (== OtherActor (Variables|Default|GetPlayerCharacterAlexReference))
    ;[1 1 1] Set the QTE's Input Key and Duration
    (Default|CreateQTE (Variables|Default|GetPlayerCharacterAlexReference) "Z" (Math|Random|RandomFloatinRange 0.5 2.0))))

(event Collision|EventActorEndOverlap
  (params (OtherActor :type Actor%20Object%20Reference))
  (bind _playercharacteralexreference (Variables|Default|GetPlayerCharacterAlexReference))
  (if (== _playercharacteralexreference OtherActor)
    (Class|CommonActivatableWidget|DeactivateWidget (Variables|/Game/Alex/BP_PlayerCharacter_Alex.BP_PlayerCharacter_Alex_C|GetCommonQteWidgetReference _playercharacteralexreference))))

(fn ConstructionScript)