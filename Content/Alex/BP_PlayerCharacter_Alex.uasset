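; Player character that runs a timed quick-time-event prototype, printing crit or normal damage results.
; CreateQTE zeroes movement acceleration, shows a key prompt widget and drains its bar with a timeline rate-scaled to the requested duration.
; AnyKey accepts only the target key, rating it crit in the bar's last quarter, otherwise normal.
; A correct press or timeline end deactivates the widget and restores movement; timing out prints normal damage.
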(event Custom|CreateQTE
  (params (TargetKey :type Key%20Structure :default "None") (Duration :type Float%20%28double-precision%29))
  ;[0.6867 1 0.6172] So they can't leave before completing QTE
  (Variables|/Script/Engine.CharacterMovementComponent|SetMaxAcceleration (Variables|Character|GetCharacterMovement) 0.0)
  ;[0.5579 0.7463 1] Create QTE Widget, make a reference and put it on-screen
  (bind _returnvalue (UserInterface|CreateWidget "/Game/Alex/WBP_CommonActivatableQTE_Test.WBP_CommonActivatableQTE_Test_C"))
  (bind _output_get (Variables|Default|SetCommonQteWidgetReference _returnvalue))
  ;[0.4397 0.4125 1] Sets the widget's position on the screen
  (Class|UserWidget|SetPositioninViewport _output_get (Variables|Default|GetQteScreenPosition) true)
  (UserInterface|Viewport|AddtoViewport _returnvalue 0)
  ;[1 0.4169 0.819] Get the InputKey as Text for Widget text
  (Default|SetQTEText (Variables|Default|GetCommonQteWidgetReference) (Class|KismetInputLibrary|KeyGetDisplayName TargetKey true))
  ;[0.7247 0.4892 1] Grab the key from event and set it as a Key value
  (Variables|Default|SetInputKey TargetKey)
  ;[1 0.491 0.4793] Set Input Key Event in progress
  (Variables|Default|SetInputKeyEventInProgress? true)
  ;[0.6867 1 0.6172] Example: 1/2=0.5 The 1 second TL plays at half speed (2 seconds)
  (Components|Timeline|SetPlayRate (Variables|Default|GetTL_Duration) (/ 1.0 Duration))
  ;[1 0.9531 0.4163] Can't do TLs in AC :(
  (bind _value (Timeline|TL_Duration PlayFromStart)
    (:Update
      ;[0.6867 1 0.6172] Access TimerBar and decrease its percent
      (Progress|SetPercent (Variables|/Game/Alex/WBP_CommonActivatableQTE_Test.WBP_CommonActivatableQTE_Test_C|GetTimerBar (Variables|Default|GetCommonQteWidgetReference)) (Math|Float|Lerp 1.0 0.0 _value)))
    (:Finished
      ;[1 0.491 0.4793] Was the Input Key Event finished before the TL finished? If not, print "normal damage"
      (if (Variables|Default|GetInputKeyEventInProgress?)
        (Development|PrintString "Normal Damage"))
      ;[1 0.491 0.4793] After TL ended, Input Key Event is no longer in progress
      (Variables|Default|SetInputKeyEventInProgress? false)
      (Class|CommonActivatableWidget|DeactivateWidget (Variables|Default|GetCommonQteWidgetReference))
      ;[0.6867 1 0.6172] Re-enable Movement after TL finishes
      (Variables|/Script/Engine.CharacterMovementComponent|SetMaxAcceleration (Variables|Character|GetCharacterMovement) 2048.0))))

(event EventBeginPlay
  (|CallParentFunction) ; This node is disabled and will not be called.\nDrag off pins to build functionality.
)

(event Input|KeyboardEvents|AnyKey
  (params (Key :type Key%20Structure :default "None"))
  (:Pressed
    ;[1 0.491 0.4793] Is the Input Key Event in progress?
    (if (Variables|Default|GetInputKeyEventInProgress?)
      ;[1 0.491 0.4793] Has the Correct Input Key been pressed?
      (if (== Key (Variables|Default|GetInputKey))
        ;[1 0.491 0.4793] Is the InputKey being pressed when the TimerBar's percent below or equal to 25%? If yes, print "Crit Damage". If no, print "Normal Damage"
        (if (<= (Variables|/Script/UMG.ProgressBar|GetPercent (Variables|/Game/Alex/WBP_CommonActivatableQTE_Test.WBP_CommonActivatableQTE_Test_C|GetTimerBar (Variables|Default|GetCommonQteWidgetReference))) 0.25)
          (Development|PrintString "Crit Damage")
          (else
            (Development|PrintString "Normal Damage")))
        ;[1 0.491 0.4793] After player attempted QTE, Input Key Event is no longer in progress
        (Variables|Default|SetInputKeyEventInProgress? false)
        (Class|CommonActivatableWidget|DeactivateWidget (Variables|Default|GetCommonQteWidgetReference))
        ;[0.6867 1 0.6172] Re-enable movement after attempting QTE event
        (Variables|/Script/Engine.CharacterMovementComponent|SetMaxAcceleration (Variables|Character|GetCharacterMovement) 2048.0)))))

(fn ConstructionScript
  (|CallParentFunction))