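; BP_Enemy_Alex is an overworld enemy that chases the player and starts a battle on contact.
; AI perception sets the blackboard TargetActor to the player when sensed, clears it when lost, and switches walk speed to move faster while sensing.
; Tick derives EnemyDirectionality from velocity, with Y inverted, for facing direction.
; The BattleTrigger overlap with the player opens the BattleTest level, marked as work in progress.
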(event OnTargetPerceptionUpdated(AIPerception)
  (params (Actor :type Actor%20Object%20Reference) (Stimulus :type AI%20Stimulus%20Structure))
  (bind _bsuccessfullysensed (Utilities|Struct|BreakAIStimulus Stimulus))
  ;[1 1 1] When the target perception is updated, compare the perceived actor to the player character. If they're equal, set the actor's value as the TargetActor key in the enemy's blackboard.
  (bind _asbp_player_character (Utilities|Casting|CastToBP_PlayerCharacter Actor))
  (if (== _asbp_player_character Actor)
    (AI|Components|Blackboard|SetValueasObject (AI|GetBlackboard 0) (Utilities|Name|MakeLiteralName "TargetActor") (select _bsuccessfullysensed _asbp_player_character 0))
    ;[1 0.491 0.4793] If an actor is successfully sensed, change the walk speed to 375. If not, change it to 300.
    (if _bsuccessfullysensed
      (Variables|/Script/Engine.CharacterMovementComponent|SetMaxWalkSpeed (Variables|Character|GetCharacterMovement) 375.0)
      (else
        (Variables|/Script/Engine.CharacterMovementComponent|SetMaxWalkSpeed (Variables|Character|GetCharacterMovement) 3e+02)))))

(event OnComponentBeginOverlap(BattleTrigger)
  (params (OverlappedComponent :type Primitive%20Component%20Object%20Reference) (OtherActor :type Actor%20Object%20Reference) (OtherComp :type Primitive%20Component%20Object%20Reference) (OtherBodyIndex :type Integer) (bFromSweep :type Boolean) (SweepResult :type Hit%20Result%20Structure%20%28by%20ref%29))
  ;[1 1 1] Triggers battle when touching the player (Work in progress)
  (if (== OtherActor (Game|GetPlayerCharacter 0))
    (Game|OpenLevel(byName) "BattleTest")))

(event EventBeginPlay
  (|CallParentFunction))

(event EventTick
  (params (DeltaSeconds :type Float%20%28single-precision%29))
  (bind _returnvalue (Transformation|GetVelocity))
  ;[1 1 1] Determines enemy facing direction
  (Variables|Default|SetEnemy%20Directionality (Math|Vector2D|MakeVector2D (.x _returnvalue) (* (.y _returnvalue) -1.0))))

(fn ConstructionScript
  (|CallParentFunction))