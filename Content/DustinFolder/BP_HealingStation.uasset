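; BP_HealingStation is an interactable that restores the player character to full HP.
; On Interact, it casts player 0's character to BP_PlayerCharacter, disables its input, heals it and plays a 2D healing jingle.
; A delay derived from the jingle's duration, ending one second short of it, then re-enables input.
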(event EventInteract
  (bind _asbp_player_character (Utilities|Casting|CastToBP_PlayerCharacter (Game|GetPlayerCharacter 0)))
  (Input|DisableInput _asbp_player_character 0)
  (Default|HealtoFullHP _asbp_player_character)
  (bind _returnvalue (Audio|SpawnSound2D "/Game/Imports/Sounds/HealingJingle.HealingJingle" 1.0 1.0 0.0 0))
  (Audio|Components|Audio|Play _returnvalue 1.0)
  (Utilities|FlowControl|Delay (- (Variables|/Script/Engine.SoundBase|GetDuration (Variables|/Script/Engine.AudioComponent|GetSound _returnvalue)) 1.0))
  (Input|EnableInput _asbp_player_character 0))

(fn ConstructionScript)