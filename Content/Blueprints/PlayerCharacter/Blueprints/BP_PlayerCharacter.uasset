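; Player character Blueprint that handles movement, interaction with actors and a full-HP heal.
; BeginPlay adds the IMC_Player Enhanced Input context, and IA_Move drives movement along fixed world axes while saving the input as Directionality.
; IA_Interact uses Directionality to run a short, debug-drawn sphere trace from the capsule, then sends InteractMessage to the hit actor.
; HealToFullHP resets current HP to the maximum.
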(event Input|EnhancedActionEvents|EnhancedInputActionIA_Move
  (params (ActionValue :type Vector%202D%20Structure) (ElapsedSeconds :type Float%20%28double-precision%29) (TriggeredSeconds :type Float%20%28double-precision%29) (InputAction :type Input%20Action%20Object%20Reference :default "/Game/Blueprints/PlayerCharacter/Blueprints/Input/IA_Move.IA_Move"))
  ;[1 1 1] Determines movement direction
  (Pawn|Input|AddMovementInput "1.000000,0.000000,0.000000" (.x ActionValue) false)
  (Pawn|Input|AddMovementInput "0.000000,-1.000000,0.000000" (.y ActionValue) false)
  (Variables|Default|SetDirectionality (Math|Vector2D|MakeVector2D (.x ActionValue) (.y ActionValue))))

(event Input|EnhancedActionEvents|EnhancedInputActionIA_Interact
  (params (ActionValue :type Boolean) (ElapsedSeconds :type Float%20%28double-precision%29) (TriggeredSeconds :type Float%20%28double-precision%29) (InputAction :type Input%20Action%20Object%20Reference :default "/Game/Blueprints/PlayerCharacter/Blueprints/Input/IA_Interact.IA_Interact"))
  (bind _capsulecomponent (Variables|Default|GetCapsuleComponent))
  (bind _returnvalue (Transformation|GetWorldLocation _capsulecomponent))
  ;[1 1 1] Draws a sphere in the direction the player is facing, then calls the Interact Interface on a hit actor
  (:Started
    (bind _outhit (Collision|SphereTraceByChannel _returnvalue (+ _returnvalue (* (Variables|Default|GetDirectionality) "50.000000,-50.000000,1.000000")) 2e+01 "TraceTypeQuery1" false 0 "ForDuration"))
    (Class|BPIInteract|Interact(Message) (.HitActor (Collision|BreakHitResult _outhit)))))

(event EventBeginPlay
  ;[1 1 1] Maps directional keys as inputs in GM_Base
  (bind _asplayer_controller (Utilities|Casting|CastToPlayerController (Pawn|GetController)))
  (Input|AddMappingContext (PlayerController|LocalPlayerSubsystems|GetEnhancedInputLocalPlayerSubsystem _asplayer_controller) "/Game/Blueprints/PlayerCharacter/Blueprints/Input/IMC_Player.IMC_Player" 0 "(bIgnoreAllPressedKeysUntilRelease=True,bForceImmediately=False,bNotifyUserSettings=False)"))

(fn ConstructionScript)

(fn HealtoFullHP
  (Variables|Default|SetCurrPlayerHP (Variables|Default|GetMaxPlayerHP)))