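; BP_SaveTest is a keyboard-driven test Blueprint for saving and loading a single number through BP_SaveGame.
; On BeginPlay it enables player input and loads TestNumber from the hardcoded "SaveOne" slot into Test, if that save exists.
; Keys increment or print Test, or write it to a newly created save object, using that object's own slot name and user index, and print the result.
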(event EventBeginPlay
  (Input|EnableInput (Game|GetPlayerController 0))
  (bind _returnvalue (SaveGame|LoadGamefromSlot "SaveOne"))
  (bind _asbp_save_game (Utilities|Casting|CastToBP_SaveGame _returnvalue))
  (Variables|Default|Settest (Variables|/Game/Mario/BP_SaveGame.BP_SaveGame_C|GetTestNumber _asbp_save_game)))

(event Input|KeyboardEvents|E
  (params (Key :type Key%20Structure :default "None"))
  (:Pressed
    (bind _result (Math|Integer|IncrementInt (Variables|Default|Gettest))
      (:%20%20
        (Development|PrintString (Utilities|String|ToString(Integer) _result))))))

(event Input|KeyboardEvents|S
  (params (Key :type Key%20Structure :default "None"))
  (:Pressed
    (bind _returnvalue (SaveGame|CreateSaveGameObject "/Game/Mario/BP_SaveGame.BP_SaveGame_C"))
    (bind _output_get (Variables|Default|SetSaveGame _returnvalue))
    (Variables|/Game/Mario/BP_SaveGame.BP_SaveGame_C|SetTestNumber _output_get (Variables|Default|Gettest))
    (bind _returnvalue_2 (SaveGame|SaveGametoSlot (Variables|Default|GetSaveGame) (Variables|/Game/Mario/BP_SaveGame.BP_SaveGame_C|GetSaveSlotName _returnvalue) (Variables|/Game/Mario/BP_SaveGame.BP_SaveGame_C|GetUserIndex _returnvalue)))
    (Development|PrintString (select _returnvalue_2 "Saved Game" "Save Failed"))))

(event Input|KeyboardEvents|1
  (params (Key :type Key%20Structure :default "None"))
  (:Pressed
    (Development|PrintString (Utilities|String|ToString(Integer) (Variables|Default|Gettest)))))

(fn ConstructionScript)